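; NPC spawner actor that repeatedly spawns an actor of the configured Spawn class around its billboard.
; BeginPlay starts a looping timer at SpawnTime intervals and stores its handle.
; Each tick of that timer spawns one actor at a random X/Y offset from the billboard, at height Z with a random yaw.
; The GetRandomPos function is an empty stub.
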(event Custom|CustomEvent_0
  (bind _returnvalue (Math|Random|RandomFloatinRange -2e+02 2e+02))
  (bind _billboard (Variables|Default|GetBillboard))
  (bind _returnvalue_2 (Transformation|GetWorldLocation _billboard))
  (Game|SpawnActorfromClass (Variables|Default|GetSpawn) (Math|Transform|MakeTransform (Math|Vector|MakeVector (+ (.x _returnvalue_2) (Math|Random|RandomFloatinRange -2e+02 2e+02)) (+ (.y _returnvalue_2) _returnvalue) (Variables|Default|GetZ)) (Math|Rotator|MakeRotator 0.0 0.0 _returnvalue) "1,1,1") "Undefined" 0 0))

(event EventBeginPlay
  (bind _returnvalue (Utilities|Time|SetTimerbyEvent (delegate Custom|CustomEvent_0) (Variables|Default|GetspawnTime) true))
  (Variables|Default|Settimer _returnvalue))

(event Collision|EventActorBeginOverlap
  (params (OtherActor :type Actor%20Object%20Reference)))

(event EventTick
  (params (DeltaSeconds :type Float%20%28single-precision%29)))

(fn ConstructionScript)

(fn GetRandomPos
  (params (center :type Transform)))