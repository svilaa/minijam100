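; Spike hazard actor that kills NPCs on overlap.
; On BeginPlay it caches the main game instance.
; When an overlapping actor has a capsule component tagged NPC, it calls Ded on the game instance with a value of one, then destroys that actor.
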(event Collision|EventActorBeginOverlap
  (params (OtherActor :type Actor%20Object%20Reference))
  (bind _returnvalue (Actor|GetComponentbyClass OtherActor "/Script/Engine.CapsuleComponent"))
  (Utilities|IsValid _returnvalue
    (:Is%20Valid
      (if (Components|ComponentHasTag _returnvalue "NPC")
        (Default|Ded (Variables|Default|GetAs%20Main%20Game%20Instance) 1)
        (Actor|DestroyActor (Components|GetOwner _returnvalue))))))

(event EventBeginPlay
  (bind _asmain_game_instance (Utilities|Casting|CastTomain_game_instance (Game|GetGameInstance)))
  (Variables|Default|SetAs%20Main%20Game%20Instance _asmain_game_instance))

(fn ConstructionScript)