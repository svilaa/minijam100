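; Wagon Blueprint that collects cargo by counting overlapping actors whose static mesh component carries the cargo tag.
; On overlap, it increments the current cargo count and destroys the cargo actor.
; Exceeding the maximum only prints an overflow message, so extra cargo is still counted and destroyed.
; Debug prints report each collision and cargo entry.
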(event Collision|EventActorBeginOverlap
  (params (OtherActor :type Actor%20Object%20Reference))
  (bind _returnvalue (Actor|GetComponentbyClass OtherActor "/Script/Engine.StaticMeshComponent"))
  (bind _componenttags (Variables|/Script/Engine.ActorComponent|GetComponentTags _returnvalue))
  ;[1 1 1] Increase Cargo Amount
  (Development|PrintString (Utilities|String|Append "Collided with" (Utilities|GetDisplayName _returnvalue) ", with tag "))
  (if (Utilities|Array|IsValidIndex _componenttags (Utilities|Array|FindItem _componenttags (Variables|Default|GetCargoTag)))
    (Development|PrintString (Utilities|String|Append "Cargo entered" (Utilities|GetDisplayName OtherActor)))
    (bind _result (Math|Integer|IncrementInt (Variables|Default|GetCurrentCargoAmount))
      (:%20%20
        (Actor|DestroyActor OtherActor)
        (Math|Integer|CompareInt _result (Variables|Default|GetMaxCargoAmount)
          (:>
            (Development|PrintString (Utilities|String|Append "Overflowing by " (Utilities|String|ToString(Integer) _result)))))))))

(fn ConstructionScript)