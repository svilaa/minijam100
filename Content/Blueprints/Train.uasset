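; Train actor that makes one timed pass through a station: it arrives, stops in the middle, departs and destroys itself.
; On BeginPlay it places its Cube component at one station edge, chosen by MoveLeft through GetLimitPos, which returns plus or minus StationWidth on relative Y.
; MoveComponentTo eases the cube into the center and, after a StopDuration delay, out to the opposite edge, printing debug messages along the way.
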(event EventBeginPlay
  (bind _returnvalue (Math|Vector|MakeVector 0.0 0.0 0.0))
  ;[1 1 1] Spawn on the correct side
  (bind _newparam (CallFunction|GetLimitPos (Variables|Default|GetMoveLeft)))
  (Development|PrintString (Utilities|String|Append "Train spawned at " (Utilities|String|ToString(Vector) _newparam)))
  (Transformation|SetRelativeLocation (Variables|Default|GetCube) _newparam false false)
  ;[1 1 1] Stop at the middle of the station
  (Components|MoveComponentTo (Variables|Default|GetCube) _returnvalue "0, 0, 0" true false (Variables|Default|GetReachMidDuration) false)
  (Development|PrintString (Utilities|String|Append "Train stopped at " (Utilities|String|ToString(Vector) _returnvalue)))
  (Utilities|FlowControl|Delay (Variables|Default|GetStopDuration))
  ;[1 1 1] Stop at the middle of the station
  (bind _newparam_2 (CallFunction|GetLimitPos (not (Variables|Default|GetMoveLeft))))
  (Components|MoveComponentTo (Variables|Default|GetCube) _newparam_2 "0, 0, 0" false true (Variables|Default|GetReachMidDuration) false)
  (Development|PrintString (Utilities|String|Append "Train destroyed at " (Utilities|String|ToString(Vector) _newparam_2)))
  (Actor|DestroyActor))

(fn ConstructionScript)

(fn GetLimitPos
  (params (RightSide :type Boolean))
  (return (Math|Vector|MakeVector 0.0 (select RightSide (- 0.0 (Variables|Default|GetStationWidth)) (Variables|Default|GetStationWidth)) 0.0)))