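; BP_Spawner is a cargo spawner that drops randomly chosen cargo types at random navigable points within a station radius, raised by a height offset.
; When enabled, BeginPlay starts a loop that spawns one cargo, logs a location and waits a random delay between configurable limits.
; The loop checks IsAlive on main_game_instance before each spawn and ends once it is false.
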(event EventBeginPlay
  (bind _heightoffset (Variables|Default|GetHeightOffset))
  (bind _cargotypes (Variables|Default|GetCargoTypes))
  (bind _stationradius (Variables|Default|GetStationRadius))
  (bind _randomlocation (Class|NavigationSystemV1|GetRandomPointinNavigableRadius (Math|Vector|MakeVector 0.0 0.0 0.0) _stationradius 0 0))
  (bind _returnvalue (+ (.z _randomlocation) _heightoffset))
  (bind _returnvalue_2 (Math|Vector|MakeVector (.x _randomlocation) (.y _randomlocation) _returnvalue))
  (if (Variables|Default|GetenabledSpawner)
    (bind _asmain_game_instance (Utilities|Casting|CastTomain_game_instance (Game|GetGameInstance)))
    (if (Variables|/Game/Blueprints/main_game_instance.main_game_instance_C|Getis_alive _asmain_game_instance) :!label _label
      (Game|SpawnActorfromClass (Utilities|Array|Get(acopy) _cargotypes (Math|Random|RandomInteger (Utilities|Array|Length _cargotypes))) (Math|Transform|MakeTransform _returnvalue_2 "0, 0, 0" "1,1,1") "Undefined" 0 0)
      (Development|PrintString (Utilities|String|Append "Spawning cargo at " (Utilities|String|ToString(Vector) _returnvalue_2)) false)
      (Utilities|FlowControl|Delay (Math|Random|RandomFloatinRange (Variables|Default|GetMinTimeBetweenSpawns) (Variables|Default|GetMaxTimeBetweenSpawns)))
      (goto _label))))

(fn ConstructionScript)