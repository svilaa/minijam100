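; BP_TrainLane is a lane actor that keeps spawning trains along it while the player is alive.
; On BeginPlay it spawns a BP_Train at its root transform, then waits for that train's full trip plus a configurable gap.
; The wait is computed from the spawned train's travel and stop durations, and the loop repeats until PlayerIsAlive is false.
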(event EventBeginPlay
  (bind _returnvalue (Game|SpawnActorfromClass "/Game/Blueprints/BP_Train.BP_Train_C" (Transformation|GetWorldTransform (Variables|Default|GetDefaultSceneRoot)) "Undefined" 0 0 :!label _label))
  (Utilities|FlowControl|Delay (+ (* (Variables|/Game/Blueprints/BP_Train.BP_Train_C|GetReachMidDuration _returnvalue) 2.0) (Variables|/Game/Blueprints/BP_Train.BP_Train_C|GetStopDuration _returnvalue) (Variables|Default|GetTimeBetweenTrains)))
  (if (Variables|Default|GetPlayerIsAlive)
    (goto _label)))

(fn ConstructionScript)