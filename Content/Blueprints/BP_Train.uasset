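; BP_Train is a train that builds itself from random wagons, passes through a station with a timed stop, then destroys itself.
; On BeginPlay it starts at one side and attaches a DifficultyManager-bounded number of wagons, spaced by mesh bounds.
; Eased moves carry it to a randomized stop and onward out.
; It then increments TrainsPassed and notifies DifficultyManager; the cargo-to-score logic is disconnected.
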(event EventBeginPlay
  (bind _wagontypes (Variables|Default|GetWagonTypes))
  (bind _defaultsceneroot (Variables|Default|GetDefaultSceneRoot))
  (bind _returnvalue (Transformation|GetWorldLocation _defaultsceneroot))
  (Utilities|FlowControl|Sequence
    (:then_0
      ;[1 1 1] Set Scene Root Position
      (bind _newparam (CallFunction|GetSidesPos (Variables|Default|GetMoveLeft)))
      (Transformation|SetWorldLocation _defaultsceneroot _newparam false false)
      (Development|PrintString (Utilities|String|Append "Moved to" (Utilities|String|ToString(Vector) _newparam))))
    (:then_1
      (bind _outactors (Actor|GetAllActorsOfClass "/Game/Blueprints/Difficulty/DifficultyManager.DifficultyManager_C"))
      (bind _maxwagons (Default|GetMaxWagons (Utilities|Array|Get(acopy) _outactors)))
      (bind _maxwagons_2 (Default|GetMinWagons (Utilities|Array|Get(acopy) _outactors)))
      ;[1 1 1] Spawn Wagons
      (for _index (range 0 (Math|Random|RandomIntegerinRange _maxwagons_2 _maxwagons))
        (bind _returnvalue_2 (Game|SpawnActorfromClass (Utilities|Array|Get(acopy) _wagontypes (Math|Random|RandomInteger (Utilities|Array|Length _wagontypes))) (Math|Transform|MakeTransform (Math|Vector|MakeVector (.x _returnvalue) (+ (.y _returnvalue) (Variables|Default|GetTrainWidth)) (.z _returnvalue))) "Undefined" 0 0))
        (Transformation|AttachComponentToComponent _returnvalue_2 _defaultsceneroot "None" "KeepWorld" "KeepRelative" "KeepRelative" true)
        (Variables|Default|SetTrainWidth (+ (Variables|Default|GetTrainWidth) (* (.y (.Max (Components|StaticMesh|GetLocalBounds (Actor|GetComponentbyClass _returnvalue_2 "/Script/Engine.StaticMeshComponent")))) 2.0) (Variables|Default|GetDistanceBetweenWagons)))))
    (:then_2
      ;[1 1 1] Stop at the middle of the station
      (bind _newparam_2 (CallFunction|GetStationMidPos))
      (Components|MoveComponentTo _defaultsceneroot _newparam_2 "0, 0, 0" true false (Variables|Default|GetReachMidDuration) false)
      (Utilities|FlowControl|Delay (Variables|Default|GetStopDuration))
      ;[1 1 1] End of station, destroy objects and send score
      (bind _newparam_3 (CallFunction|GetSidesPos (not (Variables|Default|GetMoveLeft))))
      (Components|MoveComponentTo _defaultsceneroot _newparam_3 "0, 0, 0" false true (Variables|Default|GetReachMidDuration) false)
      (Development|PrintString (Utilities|String|Append "Train destroyed at " (Utilities|String|ToString(Vector) _newparam_3)) false)
      (bind _arrayelement (Utilities|Array|ReverseforEachLoop (Actor|GetAttachedActors true))
        (:LoopBody
          (Actor|DestroyActor _arrayelement))
        (:Completed
          (bind _asmain_game_instance (Utilities|Casting|CastTomain_game_instance (Game|GetGameInstance)))
          (bind _result (Math|Integer|IncrementInt (Variables|/Game/Blueprints/main_game_instance.main_game_instance_C|Gettrains_passed _asmain_game_instance))
            (:%20%20
              (bind _outactors_2 (Actor|GetAllActorsOfClass "/Game/Blueprints/Difficulty/DifficultyManager.DifficultyManager_C"))
              (Default|OnTrainPass (Utilities|Array|Get(acopy) _outactors_2) _result)
              (Actor|DestroyActor))))))))

(fn ConstructionScript)

(fn GetSidesPos
  (params (RightSide :type Boolean))
  (bind _defaultsceneroot (Variables|Default|GetDefaultSceneRoot))
  (bind _stationwidth (Variables|Default|GetStationWidth))
  (bind _returnvalue (Transformation|GetWorldLocation _defaultsceneroot))
  (bind _returnvalue_2 (/ _stationwidth 2.0))
  (bind _result (Math|Float|NegateFloat (+ _returnvalue_2 (Variables|Default|GetTrainWidth)))
    (:%20%20
      (return (Math|Vector|MakeVector (.x _returnvalue) (+ (select RightSide _result _returnvalue_2) (.y _returnvalue)) (.z _returnvalue))))))

(fn GetStationMidPos
  (bind _stationwidth (Variables|Default|GetStationWidth))
  (bind _defaultsceneroot (Variables|Default|GetDefaultSceneRoot))
  (bind _returnvalue (/ _stationwidth 2.0))
  (bind _returnvalue_2 (Transformation|GetWorldLocation _defaultsceneroot))
  (bind _result (Math|Float|NegateFloat _returnvalue)
    (:%20%20
      (return (Math|Vector|MakeVector (.x _returnvalue_2) (+ (.y _returnvalue_2) (+ _result (Math|Random|RandomFloatinRange 0.0 (Math|Float|Clamp(Float) (- _returnvalue (Variables|Default|GetTrainWidth)) _result _returnvalue)))) (.z _returnvalue_2))))))