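; DifficultyManager tracks the game's difficulty level from the number of trains that have passed.
; On each train pass it looks up the level in the LevelByTrainsPassed threshold array and prints it to screen.
; When the level changes, it stores the new value and tells the first TopDownController found to zoom out the camera for that level.
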(event Custom|OnTrainPass
  (params (TrainsPassed :type Integer))
  ;[1 1 1] Increase Level
  (bind _level (CallFunction|GetLevel TrainsPassed))
  (Development|PrintString (Utilities|String|Append "Level " (Utilities|String|ToString(Integer) _level)))
  (if (!= _level (Variables|Default|GetCurrentLevel))
    (Variables|Default|SetCurrentLevel _level)
    (Utilities|FlowControl|Sequence
      (:then_3
        ;[1 1 1] Zoom Out Camera
        (bind _outactors (Actor|GetAllActorsOfClass "/Game/TopDownBP/Blueprints/TopDownController.TopDownController_C"))
        (Default|ZoomOutCamera (Utilities|Array|Get(acopy) _outactors) (Variables|Default|GetCurrentLevel))))))

(fn ConstructionScript)

(fn GetLevel
  (params (TrainsPassed :type Integer))
  (bind _levelbytrainspassed (Variables|Default|GetLevelByTrainsPassed))
  (bind _index (Utilities|FlowControl|ForLoopwithBreak 0 (Utilities|Array|Length _levelbytrainspassed) :!label _label)
    (:LoopBody
      (Math|Integer|CompareInt TrainsPassed (Utilities|Array|Get(acopy) _levelbytrainspassed _index)
        (:<
          (goto _label Break))))
    (:Completed
      (return (- _index 1)))))