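; TrainLane is a lane actor that repeatedly spawns Train actors at the transform of its root scene component.
; From BeginPlay it spawns a train, waits out that train's full run (twice its reach-middle time plus its stop time) and an extra gap between trains.
; It then loops back to spawn the next train while PlayerIsAlive is true, a flag this graph only reads.
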(event EventBeginPlay
  (bind _returnvalue (Game|SpawnActorfromClass "/Game/Blueprints/Train.Train_C" (Transformation|GetRelativeTransform (Variables|Default|GetDefaultSceneRoot)) "Undefined" 0 0 :!label _label))
  (Utilities|FlowControl|Delay (+ (* (Variables|/Game/Blueprints/Train.Train_C|GetReachMidDuration _returnvalue) 2.0) (Variables|/Game/Blueprints/Train.Train_C|GetStopDuration _returnvalue) (Variables|Default|GetTimeBetweenTrains)))
  (if (Variables|Default|GetPlayerIsAlive)
    (goto _label)))

(fn ConstructionScript)